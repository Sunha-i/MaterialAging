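; BP_Bake renders materials into render targets, serving as a bake utility in the Aging/Blur folder.
; Its Bake event pairs the RenderTarget and Material arrays by index, stopping at the shorter one, and draws each material into its target.
; The Construction Script calls Bake, so targets refresh whenever construction runs, while BeginPlay, overlap and Tick do nothing.
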(event `Bake`
  (for _index (range (`KismetMathLibrary.Min` (`KismetArrayLibrary.Array_Length` (`self.RenderTarget`)) (`KismetArrayLibrary.Array_Length` (`self.Material`))))
    (`KismetRenderingLibrary.DrawMaterialToRenderTarget` (`|GetArrayItem` (`self.RenderTarget`) _index) (`|GetArrayItem` (`self.Material`) _index))))

(fn `UserConstructionScript`
  (`self.Bake`))