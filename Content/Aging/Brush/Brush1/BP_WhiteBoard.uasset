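; Paintable whiteboard Blueprint that records brush marks in the PaintBoard render target.
; On BeginPlay it wraps the WhiteBoardMarker material in a dynamic instance and clears the render target to black.
; DrawOnWhiteBoard passes a 2D location to the marker's DrawLocation parameter, then stamps it with DrawMaterialToRenderTarget.
; DrawSize sets the marker's Size parameter, which applies to subsequent draws.
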(event `self.ReceiveBeginPlay`
  (bind _returnvalue (`KismetMaterialLibrary.CreateDynamicMaterialInstance` "/Game/Aging/Brush/Brush1/WhiteBoardMarker.WhiteBoardMarker"))
  (set `self.WhiteBoardMarker` _returnvalue)
  (`KismetRenderingLibrary.ClearRenderTarget2D` "/Game/Aging/Brush/Brush1/PaintBoard.PaintBoard"))

(event `DrawOnWhiteBoard`
  (params (LocationToDraw :type "Vector2D Structure"))
  (bind _whiteboardmarker (`self.WhiteBoardMarker`))
  (`MaterialInstanceDynamic.SetVectorParameterValue` _whiteboardmarker "DrawLocation" (`KismetMathLibrary.Conv_VectorToLinearColor` (`KismetMathLibrary.Conv_Vector2DToVector` LocationToDraw 0.1)))
  (`KismetRenderingLibrary.DrawMaterialToRenderTarget` "/Game/Aging/Brush/Brush1/PaintBoard.PaintBoard" _whiteboardmarker))

(event `DrawSize`
  (params (DrawSize :type "Float (double-precision)"))
  (`MaterialInstanceDynamic.SetScalarParameterValue` (`self.WhiteBoardMarker`) "Size" DrawSize))

(fn `UserConstructionScript`)