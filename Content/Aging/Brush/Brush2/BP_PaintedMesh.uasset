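; Paintable skeletal mesh actor that draws marks into a damage mask render target, cleared on BeginPlay.
; Paint takes a position and normal, first calls UnWrap, then draws M_Paint_Texture with those parameters into CRT_DamageMask.
; UnWrap captures only the mesh through a SceneCapture2D, temporarily swapping slot 0 to M_UnWrap and restoring the original materials afterwards.
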(event `self.ReceiveBeginPlay`
  (`KismetRenderingLibrary.ClearRenderTarget2D` "/Game/Aging/Brush/Brush2/CRT_DamageMask.CRT_DamageMask"))

(fn `Paint`
  (params (Position :type "Vector Structure") (Normal :type "Vector Structure"))
  (`self.UnWrap`)
  (bind _returnvalue (`KismetMaterialLibrary.CreateDynamicMaterialInstance` "/Game/Aging/Brush/Brush2/M_Paint_Texture.M_Paint_Texture"))
  (`MaterialInstanceDynamic.SetVectorParameterValue` _returnvalue "Position" (`KismetMathLibrary.Conv_VectorToLinearColor` Position))
  (`MaterialInstanceDynamic.SetVectorParameterValue` _returnvalue "Normal" (`KismetMathLibrary.Conv_VectorToLinearColor` Normal))
  (`KismetRenderingLibrary.DrawMaterialToRenderTarget` "/Game/Aging/Brush/Brush2/CRT_DamageMask.CRT_DamageMask" _returnvalue))

(fn `UnWrap`
  (locals (TmpMaterials :type "Array of MaterialInterface Object Reference"))
  (bind _scenecapturecomponent2d (`self.SceneCaptureComponent2D`))
  (bind _skeletalmesh (`self.SkeletalMesh`))
  (`SceneComponent.K2_SetWorldRotation` _scenecapturecomponent2d (struct :`Pitch` -90.0 :`Yaw` -90.0) false false)
  (`SceneCaptureComponent.ShowOnlyComponent` _scenecapturecomponent2d _skeletalmesh)
  (set `local.TmpMaterials` (`MeshComponent.GetMaterials` _skeletalmesh))
  (`PrimitiveComponent.SetMaterial` (`self.SkeletalMesh`) 0 "/Game/Aging/Brush/Brush2/M_UnWrap.M_UnWrap")
  (`SceneCaptureComponent2D.CaptureScene` (`self.SceneCaptureComponent2D`))
  (for (_array_element _array_index) (`local.TmpMaterials`)
    (`PrimitiveComponent.SetMaterial` (`self.SkeletalMesh`) _array_index _array_element)))

(fn `UserConstructionScript`)