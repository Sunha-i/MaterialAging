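; BP_PaintedTable is a paintable table actor that clears its damage-mask render target on BeginPlay.
; UnWrap briefly swaps the mesh's first material to M_UnWrap for a scene capture of that mesh alone, then restores the originals.
; Paint currently only draws a debug arrow along the given normal.
; Its intended chain, unwrapping then drawing M_Paint_Texture into the mask, is disconnected and uses zeroed position and normal.
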(event `self.ReceiveBeginPlay`
  (`KismetRenderingLibrary.ClearRenderTarget2D` "/Game/Aging/Brush/Brush2/CRT_DamageMask.CRT_DamageMask"))

(fn `Paint`
  (params (Position :type "Vector Structure") (Normal :type "Vector Structure"))
  (`KismetSystemLibrary.DrawDebugArrow` (0.0 0.0 0.0) (+ Position (* Normal 50.0)) 1.0 (struct :`G` 0.912548 :`B` 1.0 :`A` 1.0) 3.0 2.0))

(fn `UnWrap`
  (locals (TmpMaterials :type "Array of MaterialInterface Object Reference"))
  (bind _scenecapturecomponent2d (`self.SceneCaptureComponent2D`))
  (bind _staticmesh (`self.StaticMesh`))
  (`SceneComponent.K2_SetWorldRotation` _scenecapturecomponent2d (struct :`Pitch` -90.0 :`Yaw` -90.0) false false)
  (`SceneCaptureComponent.ShowOnlyComponent` _scenecapturecomponent2d _staticmesh)
  (set `local.TmpMaterials` (`MeshComponent.GetMaterials` _staticmesh))
  (`PrimitiveComponent.SetMaterial` (`self.StaticMesh`) 0 "/Game/Aging/Brush/Brush2/M_UnWrap.M_UnWrap")
  (`SceneCaptureComponent2D.CaptureScene` (`self.SceneCaptureComponent2D`))
  (for (_array_element _array_index) (`local.TmpMaterials`)
    (`PrimitiveComponent.SetMaterial` (`self.StaticMesh`) _array_index _array_element)))

(fn `UserConstructionScript`)