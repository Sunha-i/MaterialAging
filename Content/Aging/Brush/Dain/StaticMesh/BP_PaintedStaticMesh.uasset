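; BP_PaintedStaticMesh is a static mesh that gets painted at given positions into a damage mask render target, cleared on BeginPlay.
; Unwrap briefly swaps material slot 0 to MT_Unwrap_static, scene-captures only that mesh, then restores the materials.
; Paint draws a debug arrow, calls Unwrap, then draws a dynamic unwrap-material instance into CRT_DamageMask.
; That instance's Normal parameter receives Position, leaving the Normal input debug-only.
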(event `self.ReceiveBeginPlay`
  (`KismetRenderingLibrary.ClearRenderTarget2D` "/Game/Aging/Brush/Dain/CRT_DamageMask.CRT_DamageMask"))

(fn `Paint`
  (params (Position :type "Vector Structure") (Normal :type "Vector Structure"))
  (`KismetSystemLibrary.DrawDebugArrow` Position (+ Position (* Normal (50.0 50.0 50.0))) 1.0 (struct :`G` 1.0 :`B` 0.913426 :`A` 1.0) 1.0 1.0)
  (`self.Unwrap`)
  (bind _returnvalue (`KismetMaterialLibrary.CreateDynamicMaterialInstance` "/Game/Aging/Brush/Dain/StaticMesh/MT_Unwrap_static.MT_Unwrap_static"))
  (`MaterialInstanceDynamic.SetVectorParameterValue` _returnvalue "Position" (`KismetMathLibrary.Conv_VectorToLinearColor` Position))
  (`MaterialInstanceDynamic.SetVectorParameterValue` _returnvalue "Normal" (`KismetMathLibrary.Conv_VectorToLinearColor` Position))
  (`KismetRenderingLibrary.DrawMaterialToRenderTarget` "/Game/Aging/Brush/Dain/CRT_DamageMask.CRT_DamageMask" _returnvalue))

(fn `Unwrap`
  (locals (TempMaterials :type "Array of MaterialInterface Object Reference"))
  (bind _staticmesh (`self.StaticMesh`))
  (bind _scenecapturecomponent2d (`self.SceneCaptureComponent2D`))
  (`SceneComponent.K2_SetWorldRotation` _scenecapturecomponent2d (struct :`Pitch` -90.0 :`Yaw` -90.0) false false)
  (`SceneCaptureComponent.ShowOnlyComponent` _scenecapturecomponent2d _staticmesh)
  (set `local.TempMaterials` (`MeshComponent.GetMaterials` _staticmesh))
  (`PrimitiveComponent.SetMaterial` _staticmesh 0 "/Game/Aging/Brush/Dain/StaticMesh/MT_Unwrap_static.MT_Unwrap_static")
  (`SceneCaptureComponent2D.CaptureScene` (`self.SceneCaptureComponent2D`))
  (for (_array_element _array_index) (`local.TempMaterials`)
    (`PrimitiveComponent.SetMaterial` (`self.StaticMesh`) _array_index _array_element)))

(fn `UserConstructionScript`)